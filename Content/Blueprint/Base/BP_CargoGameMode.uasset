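; BP_CargoGameMode is the cargo game mode, which visualizes the cargo space as a 3D grid of debug boxes on BeginPlay.
; It first reads the block spacing from the Block_OffsetSize row of the DT_Float data table.
; Nested loops over the truncated CargoSize axes then draw a long-lived red box per cell, positioned from index 1 and slightly inset to separate neighbors.
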(event `self.ReceiveBeginPlay`
  (bind (_cargosize_x _cargosize_y _cargosize_z) (`KismetMathLibrary.BreakVector` (`self.CargoSize`)))
  (`parent.ReceiveBeginPlay`)
  (`|ExecutionSequence`
    (:`then_0`
      (bind _returnvalue (`|GetDataTableRow` "/Game/Blueprint/DataTable/DT_Float.DT_Float" "Block_OffsetSize")
        (:`then`
          (set `self.BlockOffsetSize` (`.Value_7_62A20CC948C6D5A8F9151E9A3ACCF9D2` (break `/Game/Blueprint/DataTable/SFloat` _returnvalue))))))
    (:`then_1`
      (for _index (range 1 (+ (`KismetMathLibrary.FTrunc` _cargosize_x) 1))
        (for _index_2 (range 1 (+ (`KismetMathLibrary.FTrunc` _cargosize_y) 1))
          (for _index_3 (range 1 (+ (`KismetMathLibrary.FTrunc` _cargosize_z) 1))
            (`KismetSystemLibrary.DrawDebugBox` (`KismetMathLibrary.MakeVector` (* _index (`self.BlockOffsetSize`)) (* _index_2 (`self.BlockOffsetSize`)) (* _index_3 (`self.BlockOffsetSize`))) (* (1.0 1.0 1.0) (* (`self.BlockOffsetSize`) 0.45)) (struct :`R` 1.0 :`A` 1.0) (struct) 999.0)))))))

(fn `UserConstructionScript`)