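; BP_Cargo is a cargo Blueprint that assembles its shape from small static mesh blocks.
; The construction script walks the nested PosInfo array, treating each outer entry as a vertical layer and each inner entry as an X/Y grid cell.
; It adds a downscaled mesh component per cell, spaced by BlockOffset on all three axes.
; The event graph holds no active logic.
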(fn `UserConstructionScript`
  (bind _blockoffset (`self.BlockOffset`))
  (for (_array_element _array_index) (`self.PosInfo`)
    (for _array_element_2 (`.PosInfo_4_D4D035944CC2E87273826AAF778DDE63` (break `/Game/Blueprint/Base/SCargoLayerInfo` _array_element))
      (bind (_x _y) (`KismetMathLibrary.BreakVector2D` _array_element_2))
      (`AddComponent|NODE_AddStaticMeshComponent-0` :`RelativeTransform` (`KismetMathLibrary.MakeTransform` (`KismetMathLibrary.MakeVector` (* _x _blockoffset) (* _y _blockoffset) (* _array_index _blockoffset)) (struct) (0.1 0.1 0.1))))))