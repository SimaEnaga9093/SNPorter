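; BP_CargoBase is a base Blueprint for cargo that builds its shape from blocks at BeginPlay.
; It reads the block spacing from DT_Float and its layout from the DT_CargoInfo row named by CargoInfoRowName.
; If that name is set, it adds a static mesh component for each layer position, scaling grid X/Y and layer index by the spacing to place blocks in stacked layers.
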(event `self.ReceiveBeginPlay`
  (bind _blockoffsetsize (`self.BlockOffsetSize`))
  (`parent.ReceiveBeginPlay`)
  (`|ExecutionSequence`
    (:`then_0`
      (bind _returnvalue (`|GetDataTableRow` "/Game/Blueprint/DataTable/DT_Float.DT_Float" "Block_OffsetSize")
        (:`then`
          (set `self.BlockOffsetSize` (`.Value_7_62A20CC948C6D5A8F9151E9A3ACCF9D2` (break `/Game/Blueprint/DataTable/SFloat` _returnvalue)))
          (bind _returnvalue_2 (`|GetDataTableRow` "/Game/Blueprint/DataTable/DT_CargoInfo.DT_CargoInfo" (`self.CargoInfoRowName`))
            (:`then`
              (set `self.CargoInfo` _returnvalue_2))))))
    (:`then_1`
      (if (!= (`self.CargoInfoRowName`) "None")
        (for (_array_element _array_index) (`.CargoLayerInfo_7_3A07D4D64D846BFD1C8EBB8C8953CB02` (break `/Game/Blueprint/DataTable/SCargoInfo` (`self.CargoInfo`)))
          (for _array_element_2 (`.PosInfo_4_D4D035944CC2E87273826AAF778DDE63` (break `/Game/Blueprint/Base/SCargoLayerInfo` _array_element))
            (bind (_x _y) (`KismetMathLibrary.BreakVector2D` _array_element_2))
            (`AddComponent|NODE_AddStaticMeshComponent-1` :`RelativeTransform` (`KismetMathLibrary.MakeTransform` (`KismetMathLibrary.MakeVector` (* _x _blockoffsetsize) (* _y _blockoffsetsize) (* _array_index _blockoffsetsize))))))))))

(fn `UserConstructionScript`)